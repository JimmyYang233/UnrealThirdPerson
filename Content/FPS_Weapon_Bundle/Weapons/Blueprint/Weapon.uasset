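; Base weapon actor from an FPS weapon bundle that handles firing checks, shot effects and outline highlighting.
; BeginPlay hides the magazine bone on the Main mesh, and CanShoot requires HasClip plus a valid Mag with bullets left.
; Shoot plays a 2D sound, decrements the Mag's bullet count and launches a physics shell casing from the ejectStart socket.
; StartHighlight and StopHighlight toggle custom depth rendering on Main.
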(event `self.ReceiveBeginPlay`
  (`SkinnedMeshComponent.HideBoneByName` (`self.Main`) "b_gun_mag" "PBO_None"))

(event `/Game/高亮material/highlineInterface.StartHighlight`
  (`PrimitiveComponent.SetRenderCustomDepth` (`self.Main`) true))

(event `/Game/高亮material/highlineInterface.StopHighlight`
  (`PrimitiveComponent.SetRenderCustomDepth` (`self.Main`) false))

(fn `canShoot`
  (returns (canShoot :type Boolean))
  (locals (`canShoot?` :type Boolean :default false))
  (bind _mag (`self.Mag`))
  (`/Engine/EditorBlueprintResources/StandardMacros.IsValid` _mag
    (:`Is Valid`
      (set `local.canShoot?` (and (`self.HasClip`) (> (`/Game/FPS_Weapon_Bundle/Weapons/Blueprint/Mag.NumberOfBullet` _mag) 0))))
    (:`Is Not Valid`
      (set `local.canShoot?` false)))
  (return (`local.canShoot?`)))

(fn `Shoot`
  (bind _main (`self.Main`))
  (bind _mag (`self.Mag`))
  (`GameplayStatics.PlaySound2D` "/Game/StarterContent/Audio/Explosion02.Explosion02" 1.0 1.0 0.0 null null)
  (set `/Game/FPS_Weapon_Bundle/Weapons/Blueprint/Mag.NumberOfBullet` (- (`/Game/FPS_Weapon_Bundle/Weapons/Blueprint/Mag.NumberOfBullet` _mag) 1) _mag)
  (bind _returnvalue (`|SpawnActorFromClass` "/Game/FPS_Weapon_Bundle/Weapons/Blueprint/Ammo_Empty.Ammo_Empty_C" (`SceneComponent.GetSocketTransform` _main "ejectStart" "RTS_World") "Undefined" "OverrideRootScale" null null))
  (`PrimitiveComponent.SetPhysicsLinearVelocity` (`/Game/FPS_Weapon_Bundle/Weapons/Blueprint/Ammo_Empty.Ammo` _returnvalue) (* (`SceneComponent.GetForwardVector` _main) (* -1.0 (`self.eject speed`))) false "None"))

(fn `UserConstructionScript`)