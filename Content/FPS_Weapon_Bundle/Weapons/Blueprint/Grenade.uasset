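; Grenade actor that explodes after a configurable delay once startCounting is called, spawning an explosion effect and sound at its location.
; A debug-drawn sphere trace then finds PUBG_MAINPLAYER hits and directly subtracts Health, with heavier damage inside half the radius, printing the result.
; The actor destroys itself afterwards.
; StartHighlight and StopHighlight toggle custom depth rendering on the grenade component for highlighting.
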(event `startCounting`
  (bind _returnvalue (`self.K2_GetActorLocation`))
  (`KismetSystemLibrary.Delay` (`self.delaySecond`))
  (`GameplayStatics.SpawnEmitterAtLocation` "/Game/StarterContent/Particles/P_Explosion.P_Explosion" _returnvalue)
  (`GameplayStatics.PlaySoundAtLocation` "/Game/StarterContent/Audio/Explosion_Cue.Explosion_Cue" _returnvalue (struct) 1.0 1.0 0.0 null null null)
  (`|ExecutionSequence`
    (:`then_0`
      (bind _outhits (`KismetSystemLibrary.SphereTraceMulti` :`Start` _returnvalue :`End` _returnvalue :`Radius` (`self.explostion radius`) :`TraceChannel` "TraceTypeQuery5" :`DrawDebugType` "ForDuration"))
      (for _array_element _outhits
        (bind (_bblockinghit _binitialoverlap _time _distance _location _impactpoint _normal _impactnormal _physmat _hitactor _hitcomponent _hitbonename _hititem _faceindex _tracestart _traceend) (`GameplayStatics.BreakHitResult` _array_element))
        (bind _aspubg_mainplayer (cast `/Game/Player/PUBG_MAINPLAYER` _hitactor))
        (if (< (`KismetMathLibrary.VSize` (- _impactpoint _traceend)) (/ (`self.explostion radius`) 2.0))
          (bind _health (`/Game/Player/PUBG_MAINPLAYER.Health` _aspubg_mainplayer))
          (bind _output_get (set `/Game/Player/PUBG_MAINPLAYER.Health` (- _health 10.0) _aspubg_mainplayer))
          (else
            (bind _output_get_2 (set `/Game/Player/PUBG_MAINPLAYER.Health` (- _health 5.0) _aspubg_mainplayer))))
        (`KismetSystemLibrary.PrintString` (`KismetStringLibrary.Conv_DoubleToString` _output_get_2)))
      (`self.K2_DestroyActor`))))

(event `self.ReceiveBeginPlay`)

(event `/Game/高亮material/highlineInterface.StartHighlight`
  (`PrimitiveComponent.SetRenderCustomDepth` (`self.Grenade`) true))

(event `/Game/高亮material/highlineInterface.StopHighlight`
  (`PrimitiveComponent.SetRenderCustomDepth` (`self.Grenade`) false))

(fn `UserConstructionScript`)