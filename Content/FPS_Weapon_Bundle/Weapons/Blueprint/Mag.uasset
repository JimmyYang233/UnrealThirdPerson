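; Mag is a weapon magazine Blueprint whose static mesh reflects whether it still holds bullets.
; Every tick it checks the bullet count and swaps to the empty magazine mesh when the count reaches zero.
; Highlight start and stop events toggle custom depth rendering on the mesh.
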(event `self.ReceiveTick`
  (params (DeltaSeconds :type "Float (single-precision)"))
  (if (== (`self.NumberOfBullet`) 0)
    (`StaticMeshComponent.SetStaticMesh` (`self.Mag`) (`self.MagEmpty`))))

(event `/Game/高亮material/highlineInterface.StartHighlight`
  (`PrimitiveComponent.SetRenderCustomDepth` (`self.Mag`) true))

(event `/Game/高亮material/highlineInterface.StopHighlight`
  (`PrimitiveComponent.SetRenderCustomDepth` (`self.Mag`) false))

(fn `UserConstructionScript`)